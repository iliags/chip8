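; Player pawn that serves as the 16-key hex keypad for the device owned by the level's C8Visualizer, apparently a CHIP-8 emulator.
; On BeginPlay it installs IMC_Default as the only Enhanced Input mapping context and caches the first C8Visualizer found.
; Each key's input action forwards both Triggered and Completed values to the device's SetKeyState.
; Space bar prints the device's VRAM string for debugging.
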(event Input|EnhancedActionEvents|EnhancedInputActionIA_0
  (params (ActionValue :type Boolean) (ElapsedSeconds :type Float%20%28double-precision%29) (TriggeredSeconds :type Float%20%28double-precision%29) (InputAction :type Input%20Action%20Object%20Reference :default "/Game/Input/Actions/IA_0.IA_0"))
  (:Triggered
    (Class|C8Device|SetKeyState (Variables|/Script/Chip8.C8Visualizer|GetDevice (Variables|Default|GetVisualizer)) "Key0" ActionValue :!label _label))
  (:Completed
    (goto _label)))

(event Input|EnhancedActionEvents|EnhancedInputActionIA_9
  (params (ActionValue :type Boolean) (ElapsedSeconds :type Float%20%28double-precision%29) (TriggeredSeconds :type Float%20%28double-precision%29) (InputAction :type Input%20Action%20Object%20Reference :default "/Game/Input/Actions/IA_9.IA_9"))
  (:Triggered
    (Class|C8Device|SetKeyState (Variables|/Script/Chip8.C8Visualizer|GetDevice (Variables|Default|GetVisualizer)) "Key9" ActionValue :!label _label))
  (:Completed
    (goto _label)))

(event Input|EnhancedActionEvents|EnhancedInputActionIA_A
  (params (ActionValue :type Boolean) (ElapsedSeconds :type Float%20%28double-precision%29) (TriggeredSeconds :type Float%20%28double-precision%29) (InputAction :type Input%20Action%20Object%20Reference :default "/Game/Input/Actions/IA_A.IA_A"))
  (:Triggered
    (Class|C8Device|SetKeyState (Variables|/Script/Chip8.C8Visualizer|GetDevice (Variables|Default|GetVisualizer)) "KeyA" ActionValue :!label _label))
  (:Completed
    (goto _label)))

(event Input|EnhancedActionEvents|EnhancedInputActionIA_B
  (params (ActionValue :type Boolean) (ElapsedSeconds :type Float%20%28double-precision%29) (TriggeredSeconds :type Float%20%28double-precision%29) (InputAction :type Input%20Action%20Object%20Reference :default "/Game/Input/Actions/IA_B.IA_B"))
  (:Triggered
    (Class|C8Device|SetKeyState (Variables|/Script/Chip8.C8Visualizer|GetDevice (Variables|Default|GetVisualizer)) "KeyB" ActionValue :!label _label))
  (:Completed
    (goto _label)))

(event Input|EnhancedActionEvents|EnhancedInputActionIA
  (params (ActionValue :type Boolean) (ElapsedSeconds :type Float%20%28double-precision%29) (TriggeredSeconds :type Float%20%28double-precision%29) (InputAction :type Input%20Action%20Object%20Reference :default "/Game/Input/Actions/IA_C.IA_C"))
  (:Triggered
    (Class|C8Device|SetKeyState (Variables|/Script/Chip8.C8Visualizer|GetDevice (Variables|Default|GetVisualizer)) "KeyC" ActionValue :!label _label))
  (:Completed
    (goto _label)))

(event Input|EnhancedActionEvents|EnhancedInputActionIA_D
  (params (ActionValue :type Boolean) (ElapsedSeconds :type Float%20%28double-precision%29) (TriggeredSeconds :type Float%20%28double-precision%29) (InputAction :type Input%20Action%20Object%20Reference :default "/Game/Input/Actions/IA_D.IA_D"))
  (:Triggered
    (Class|C8Device|SetKeyState (Variables|/Script/Chip8.C8Visualizer|GetDevice (Variables|Default|GetVisualizer)) "KeyD" ActionValue :!label _label))
  (:Completed
    (goto _label)))

(event Input|EnhancedActionEvents|EnhancedInputActionIA_E
  (params (ActionValue :type Boolean) (ElapsedSeconds :type Float%20%28double-precision%29) (TriggeredSeconds :type Float%20%28double-precision%29) (InputAction :type Input%20Action%20Object%20Reference :default "/Game/Input/Actions/IA_E.IA_E"))
  (:Triggered
    (Class|C8Device|SetKeyState (Variables|/Script/Chip8.C8Visualizer|GetDevice (Variables|Default|GetVisualizer)) "KeyE" ActionValue :!label _label))
  (:Completed
    (goto _label)))

(event Input|EnhancedActionEvents|EnhancedInputActionIA_F
  (params (ActionValue :type Boolean) (ElapsedSeconds :type Float%20%28double-precision%29) (TriggeredSeconds :type Float%20%28double-precision%29) (InputAction :type Input%20Action%20Object%20Reference :default "/Game/Input/Actions/IA_F.IA_F"))
  (:Triggered
    (Class|C8Device|SetKeyState (Variables|/Script/Chip8.C8Visualizer|GetDevice (Variables|Default|GetVisualizer)) "KeyF" ActionValue :!label _label))
  (:Completed
    (goto _label)))

(event Input|EnhancedActionEvents|EnhancedInputActionIA_1
  (params (ActionValue :type Boolean) (ElapsedSeconds :type Float%20%28double-precision%29) (TriggeredSeconds :type Float%20%28double-precision%29) (InputAction :type Input%20Action%20Object%20Reference :default "/Game/Input/Actions/IA_1.IA_1"))
  (:Triggered
    (Class|C8Device|SetKeyState (Variables|/Script/Chip8.C8Visualizer|GetDevice (Variables|Default|GetVisualizer)) "Key1" ActionValue :!label _label))
  (:Completed
    (goto _label)))

(event Input|EnhancedActionEvents|EnhancedInputActionIA_2
  (params (ActionValue :type Boolean) (ElapsedSeconds :type Float%20%28double-precision%29) (TriggeredSeconds :type Float%20%28double-precision%29) (InputAction :type Input%20Action%20Object%20Reference :default "/Game/Input/Actions/IA_2.IA_2"))
  (:Triggered
    (Class|C8Device|SetKeyState (Variables|/Script/Chip8.C8Visualizer|GetDevice (Variables|Default|GetVisualizer)) "Key2" ActionValue :!label _label))
  (:Completed
    (goto _label)))

(event Input|EnhancedActionEvents|EnhancedInputActionIA_3
  (params (ActionValue :type Boolean) (ElapsedSeconds :type Float%20%28double-precision%29) (TriggeredSeconds :type Float%20%28double-precision%29) (InputAction :type Input%20Action%20Object%20Reference :default "/Game/Input/Actions/IA_3.IA_3"))
  (:Triggered
    (Class|C8Device|SetKeyState (Variables|/Script/Chip8.C8Visualizer|GetDevice (Variables|Default|GetVisualizer)) "Key3" ActionValue :!label _label))
  (:Completed
    (goto _label)))

(event Input|EnhancedActionEvents|EnhancedInputActionIA_4
  (params (ActionValue :type Boolean) (ElapsedSeconds :type Float%20%28double-precision%29) (TriggeredSeconds :type Float%20%28double-precision%29) (InputAction :type Input%20Action%20Object%20Reference :default "/Game/Input/Actions/IA_4.IA_4"))
  (:Triggered
    (Class|C8Device|SetKeyState (Variables|/Script/Chip8.C8Visualizer|GetDevice (Variables|Default|GetVisualizer)) "Key4" ActionValue :!label _label))
  (:Completed
    (goto _label)))

(event Input|EnhancedActionEvents|EnhancedInputActionIA_5
  (params (ActionValue :type Boolean) (ElapsedSeconds :type Float%20%28double-precision%29) (TriggeredSeconds :type Float%20%28double-precision%29) (InputAction :type Input%20Action%20Object%20Reference :default "/Game/Input/Actions/IA_5.IA_5"))
  (:Triggered
    (Class|C8Device|SetKeyState (Variables|/Script/Chip8.C8Visualizer|GetDevice (Variables|Default|GetVisualizer)) "Key5" ActionValue :!label _label))
  (:Completed
    (goto _label)))

(event Input|EnhancedActionEvents|EnhancedInputActionIA_6
  (params (ActionValue :type Boolean) (ElapsedSeconds :type Float%20%28double-precision%29) (TriggeredSeconds :type Float%20%28double-precision%29) (InputAction :type Input%20Action%20Object%20Reference :default "/Game/Input/Actions/IA_6.IA_6"))
  (:Triggered
    (Class|C8Device|SetKeyState (Variables|/Script/Chip8.C8Visualizer|GetDevice (Variables|Default|GetVisualizer)) "Key6" ActionValue :!label _label))
  (:Completed
    (goto _label)))

(event Input|EnhancedActionEvents|EnhancedInputActionIA_7
  (params (ActionValue :type Boolean) (ElapsedSeconds :type Float%20%28double-precision%29) (TriggeredSeconds :type Float%20%28double-precision%29) (InputAction :type Input%20Action%20Object%20Reference :default "/Game/Input/Actions/IA_7.IA_7"))
  (:Triggered
    (Class|C8Device|SetKeyState (Variables|/Script/Chip8.C8Visualizer|GetDevice (Variables|Default|GetVisualizer)) "Key7" ActionValue :!label _label))
  (:Completed
    (goto _label)))

(event Input|EnhancedActionEvents|EnhancedInputActionIA_8
  (params (ActionValue :type Boolean) (ElapsedSeconds :type Float%20%28double-precision%29) (TriggeredSeconds :type Float%20%28double-precision%29) (InputAction :type Input%20Action%20Object%20Reference :default "/Game/Input/Actions/IA_8.IA_8"))
  (:Triggered
    (Class|C8Device|SetKeyState (Variables|/Script/Chip8.C8Visualizer|GetDevice (Variables|Default|GetVisualizer)) "Key8" ActionValue :!label _label))
  (:Completed
    (goto _label)))

(event EventBeginPlay
  (Utilities|FlowControl|Sequence
    (:then_0
      (bind _asplayer_controller (Utilities|Casting|CastToPlayerController (Pawn|GetController)))
      (Class|EnhancedInputSubsystemInterface|ClearAllMappings (PlayerController|LocalPlayerSubsystems|GetEnhancedInputLocalPlayerSubsystem _asplayer_controller))
      (Input|AddMappingContext (PlayerController|LocalPlayerSubsystems|GetEnhancedInputLocalPlayerSubsystem _asplayer_controller) "/Game/Input/IMC_Default.IMC_Default" 0 "(bIgnoreAllPressedKeysUntilRelease=True,bForceImmediately=False,bNotifyUserSettings=False)"))
    (:then_1
      (bind _outactors (Actor|GetAllActorsOfClass "/Script/Chip8.C8Visualizer"))
      (Variables|Default|SetVisualizer (Utilities|Array|Get(acopy) _outactors)))))

(event Input|KeyboardEvents|SpaceBar
  (params (Key :type Key%20Structure :default "None"))
  (:Pressed
    (Development|PrintString (Class|C8Device|GetVRAMString (Variables|/Script/Chip8.C8Visualizer|GetDevice (Variables|Default|GetVisualizer))))))

(fn ConstructionScript)